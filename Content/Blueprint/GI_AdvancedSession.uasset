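; Game instance Blueprint, judging by its GI prefix, that hosts multiplayer sessions through an Advanced Sessions node.
; Its CreateSession event runs only on the server, publishing session name, map, country and a LAN flag as extra settings, with player count as public connections.
; The Privacy input drives the LAN option.
; On success it server-travels to the map as a listen server; clients only get a printed error.
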(event Custom|Create%20Session
  (params (Session%20Name :type String) (Map%20Name :type String) (Privacy :type Boolean) (Player%20Num :type Integer) (Country :type String))
  (if (Networking|IsServer)
    (|AdvancedSession (Utilities|Array|MakeArray (Class|AdvancedSessionsLibrary|MakeLiteralSessionPropertyString "Session Name" Session%20Name) (Class|AdvancedSessionsLibrary|MakeLiteralSessionPropertyString "Map Name" Map%20Name) (Class|AdvancedSessionsLibrary|MakeLiteralSessionPropertyString "Country" Country) (Class|AdvancedSessionsLibrary|MakeLiteralSessionPropertyBool "IsLAN?" Privacy)) (Game|GetPlayerController 0) Player%20Num 0 Privacy true false true true false false false true false true
      (:OnSuccess
        (Class|AdvancedSessionsLibrary|ServerTravel (Utilities|String|Append Map%20Name "?listen") true false)))
    (else
      (Development|PrintString "Can't create session as a client!!"))))