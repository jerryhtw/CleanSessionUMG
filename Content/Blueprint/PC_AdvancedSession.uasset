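; Player controller for the session menu flow, owning the main menu, create session, server browser, delay screen and settings widgets.
; On BeginPlay the local controller creates all five, shows the mouse cursor and, if the game instance has not entered a session, shows the delay screen briefly before the main menu.
; Enum-driven show and hide events switch widgets, and another event sets the view target to a given cine camera.
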(event Custom|Show%20Widget
  (params (Widget :type E_MainMenuWidgets%20Enum :default "NewEnumerator0"))
  (if (Pawn|IsLocalPlayerController)
    (switch Utilities|FlowControl|Switch|SwitchonE_MainMenuWidgets Widget
      (:NewEnumerator0
        (UserInterface|Viewport|AddtoViewport (Variables|Default|GetWBP_MainMenu) 0))
      (:NewEnumerator1
        (UserInterface|Viewport|AddtoViewport (Variables|Default|GetWBP_Create%20Session) 0))
      (:NewEnumerator2
        (UserInterface|Viewport|AddtoViewport (Variables|Default|GetWBP_ServerBrowser) 0))
      (:NewEnumerator4
        (UserInterface|Viewport|AddtoViewport (Variables|Default|GetWBP_Delay%20Screen) 0))
      (:NewEnumerator5
        (UserInterface|Viewport|AddtoViewport (Variables|Default|GetWBP_Settings) 0)))))

(event Custom|Hide%20Widget
  (params (WIdget :type E_MainMenuWidgets%20Enum :default "NewEnumerator0"))
  (if (Pawn|IsLocalPlayerController)
    (switch Utilities|FlowControl|Switch|SwitchonE_MainMenuWidgets WIdget
      (:NewEnumerator0
        (bind _wbp_mainmenu (Variables|Default|GetWBP_MainMenu)
          (:then
            (Widget|RemovefromParent _wbp_mainmenu))
          (:else)))
      (:NewEnumerator1
        (bind _wbp_create_session (Variables|Default|GetWBP_Create%20Session)
          (:then
            (Widget|RemovefromParent _wbp_create_session))
          (:else)))
      (:NewEnumerator2
        (bind _wbp_serverbrowser (Variables|Default|GetWBP_ServerBrowser)
          (:then
            (Widget|RemovefromParent _wbp_serverbrowser))
          (:else)))
      (:NewEnumerator4
        (bind _wbp_delay_screen (Variables|Default|GetWBP_Delay%20Screen)
          (:then
            (Widget|RemovefromParent _wbp_delay_screen))
          (:else)))
      (:NewEnumerator5
        (bind _wbp_settings (Variables|Default|GetWBP_Settings)
          (:then
            (Widget|RemovefromParent _wbp_settings))
          (:else))))))

(event Custom|SetClientViewTarget
  (params (FixedCineCamera :type Cine%20Camera%20Actor%20Object%20Reference))
  (Game|Player|SetViewTargetwithBlend (Game|GetPlayerController 0) FixedCineCamera 0.0 "VTBlend_Linear" 0.0 false))

(event EventBeginPlay
  (if (Pawn|IsLocalPlayerController)
    (Utilities|FlowControl|Sequence
      (:then_0
        (bind _returnvalue (UserInterface|CreateWidget "/Game/UI/WBP_MainMenu.WBP_MainMenu_C"))
        (Variables|Default|SetWBP_MainMenu _returnvalue)
        (bind _returnvalue_2 (UserInterface|CreateWidget "/Game/UI/WBP_CreateSession.WBP_CreateSession_C"))
        (Variables|Default|SetWBP_Create%20Session _returnvalue_2)
        (bind _returnvalue_3 (UserInterface|CreateWidget "/Game/UI/WBP_ServerBrowser.WBP_ServerBrowser_C"))
        (Variables|Default|SetWBP_ServerBrowser _returnvalue_3)
        (bind _returnvalue_4 (UserInterface|CreateWidget "/Game/UI/WBP_DelayScreen.WBP_DelayScreen_C"))
        (Variables|Default|SetWBP_Delay%20Screen _returnvalue_4)
        (bind _returnvalue_5 (UserInterface|CreateWidget "/Game/UI/WBP_Settings.WBP_Settings_C"))
        (Variables|Default|SetWBP_Settings _returnvalue_5))
      (:then_1
        (Variables|Default|SetbShowMouseCursor true))
      (:then_2
        (bind _asgi_advanced_session (Utilities|Casting|CastToGI_AdvancedSession (Game|GetGameInstance)))
        (bind _output_get (Variables|Default|SetGI%20Advanced%20Session _asgi_advanced_session))
        (if (not (Variables|/Game/Blueprint/GI_AdvancedSession.GI_AdvancedSession_C|GetEnteredSession _output_get))
          (CallFunction|ShowWidget "NewEnumerator4")
          (Utilities|FlowControl|Delay 5.0)
          (CallFunction|HideWidget "NewEnumerator4")
          (CallFunction|ShowWidget "NewEnumerator0"))))))

(fn ConstructionScript)